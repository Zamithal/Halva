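; VR player controller that fades a field-of-view restriction in and out through an FOVRestrictor passed to its events.
; RestrictVision plays the restrictor's FadeIn animation partway, and UnrestrictVision plays that segment in reverse.
; MaxObscuration, clamped to 0–1 and scaled down, sets the animation end time, so it caps how obscured the view becomes.
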(event EventTick
  (params (DeltaSeconds :type Float%20%28single-precision%29)))

(event EventRestrictVision
  (params (FOV :type User%20Widget%20Object%20Reference))
  (bind _asfovrestrictor (Utilities|Casting|CastToFOVRestrictor FOV)
    (:then
      (Class|UserWidget|PlayAnimationto _asfovrestrictor (Variables|/Game/Actors/Player/FOVRestrictor.FOVRestrictor_C|GetFadeIn _asfovrestrictor) 0.0 (/ (Math|Float|Clamp(Float) (Variables|Default|GetmaxObscuration)) 4.0) 1 "Forward" 1.0))
    (:CastFailed
      (Development|PrintString "Fail"))))

(event EventUnrestrictVision
  (params (FOV :type User%20Widget%20Object%20Reference))
  (bind _asfovrestrictor (Utilities|Casting|CastToFOVRestrictor FOV))
  (Class|UserWidget|PlayAnimationto _asfovrestrictor (Variables|/Game/Actors/Player/FOVRestrictor.FOVRestrictor_C|GetFadeIn _asfovrestrictor) 0.0 (/ (Math|Float|Clamp(Float) (Variables|Default|GetmaxObscuration)) 4.0) 1 "Reverse" 1.0))

(fn ConstructionScript)