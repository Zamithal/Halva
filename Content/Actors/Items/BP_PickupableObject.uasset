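; BP_PickupableObject is a physics item that can be picked up and carried by a holder.
; SetHeld toggles mesh physics simulation, and while held, Tick snaps the actor to the valid Holder's world location and rotation via SetObjectTransform, without sweeping.
; Offset, rotation and their maintain flags have getters and setters, but the transform update does not use them.
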(event EventBeginPlay)

(event Collision|EventActorBeginOverlap
  (params (OtherActor :type Actor%20Object%20Reference)))

(event EventTick
  (params (DeltaSeconds :type Float%20%28single-precision%29))
  (bind _holder (Variables|Default|GetHolder))
  ;[1 1 1] Pickup
  (if (Variables|Default|GetHeld)
    (Utilities|IsValid _holder
      (:Is%20Valid
        (CallFunction|SetObjectTransform (Transformation|GetWorldRotation _holder) (Transformation|GetWorldLocation _holder))))))

(fn ConstructionScript
  (|CallParentFunction))

(fn SetObjectTransform
  (params (HandRotation :type Rotator) (HandLocation :type Vector))
  (Transformation|SetActorLocation HandLocation false false)
  (Transformation|SetActorRotation HandRotation))

(fn SetHeld
  (params (Held? :type Boolean))
  (Physics|SetSimulatePhysics (Variables|Default|GetStaticMeshComponent) (not Held?))
  (Variables|Default|SetHeld Held?))

(fn GetHeld
  (return (Variables|Default|GetHeld)))

(fn SetOffset
  (params (Offset :type Vector))
  (Variables|Default|SetOffset Offset))

(fn GetOffset
  (return (Variables|Default|GetOffset)))

(fn SetRotation
  (params (Rotation :type Rotator))
  (Variables|Default|SetRotation Rotation))

(fn GetRotation
  (return (Variables|Default|GetRotation)))

(fn SetMaintainRotation
  (params (MaintainRotation? :type Boolean))
  (Variables|Default|SetMaintainRotation? MaintainRotation?))

(fn GetMaintainRotation
  (return (Variables|Default|GetMaintainRotation?)))

(fn SetMaintainOffset
  (params (MaintainOffset? :type Boolean))
  (Variables|Default|SetMaintainOffset? MaintainOffset?))

(fn GetMaintainOffset
  (return (Variables|Default|GetMaintainOffset?)))

(fn SetHolder
  (params (Holder :type Static%20Mesh%20Component%20Object%20Reference))
  (Variables|Default|SetHolder Holder))

(fn GetHolder
  (return (Variables|Default|GetHolder)))